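; BP_GenericObject is a typed pickup object, such as a key or weapon, that damages enemies when thrown.
; On BeginPlay, Light and Heavy weapon types receive a random bullet count.
; Box overlaps send fixed damage to INT_BasicEnemy actors through an interface message and play impact particles and sound, without explicitly checking for a thrown state.
; Any Box hit destroys the object after a short delay.
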(event `self.ReceiveBeginPlay`
  ;[0.5052 1 0.3884] Set bullet amt only for ranged weapons
  (if (select `/Game/PickUpObject/EN_ObjectType` (`self.ObjectType`) :`NewEnumerator2` true :`NewEnumerator3` true)
    (set `self.BulletAmt` (`KismetMathLibrary.RandomIntegerInRange` 1 10))))

(event `self.Box.OnComponentHit`
  (params (HitComponent :type "PrimitiveComponent Object Reference") (OtherActor :type "Actor Object Reference") (OtherComp :type "PrimitiveComponent Object Reference") (NormalImpulse :type "Vector Structure") (Hit :type "HitResult Structure (by ref)"))
  ;[0.3831 0.7061 1] Destroy On Hit
  (`KismetSystemLibrary.Delay` 2.0)
  (`self.K2_DestroyActor`))

(event `self.Box.OnComponentBeginOverlap`
  (params (OverlappedComponent :type "PrimitiveComponent Object Reference") (OtherActor :type "Actor Object Reference") (OtherComp :type "PrimitiveComponent Object Reference") (OtherBodyIndex :type Integer) (bFromSweep :type Boolean) (SweepResult :type "HitResult Structure (by ref)"))
  (bind _returnvalue (`self.K2_GetActorLocation`))
  ;[1 0.3448 0.2817] If thrown, check overlaps
  (if (`KismetSystemLibrary.DoesImplementInterface` OtherActor "/Game/ThirdPerson/Blueprints/Interfaces/INT_BasicEnemy.INT_BasicEnemy_C")
    (message `/Game/ThirdPerson/Blueprints/Interfaces/INT_BasicEnemy.TakeDamage` OtherActor 20.0)
    (`GameplayStatics.SpawnEmitterAtLocation` "/Game/Particles/P_Impact.P_Impact" _returnvalue)
    (`GameplayStatics.PlaySoundAtLocation` "/Game/SFX/SC_MeleeHitAxe.SC_MeleeHitAxe" _returnvalue (struct) 1.0 1.0 0.0 null null null null)))

(fn `UserConstructionScript`)