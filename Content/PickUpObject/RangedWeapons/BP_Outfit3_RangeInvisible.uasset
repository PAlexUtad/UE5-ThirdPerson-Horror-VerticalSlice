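; Ranged weapon Blueprint for Outfit 3 that fires a hitscan blaster shot with a muzzle flash and sound.
; Shoot traces from the strafe camera toward the camera aim, or character forward in fixed-cam mode, then re-traces from the muzzle toward that point to correct parallax.
; Hit actors implementing INT_BasicEnemy receive ranged damage, and any hit spawns an impact emitter aligned to the surface normal.
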(event `self.ReceiveBeginPlay`
  (`parent.ReceiveBeginPlay`)
  (set `self.ShootSound` "/Game/SFX/SC_BlasterShot.SC_BlasterShot"))

(event `/Game/PickUpObject/RangedWeapons/INT_Weapon.Shoot`
  (bind _as_bp_third_person_character (`self.As BP Third Person Character`))
  (bind _returnvalue (`SceneComponent.K2_GetComponentLocation` (`self.Strafe Camera`)))
  ;[1 0.4908 0.3605] Shoot
  (`GameplayStatics.SpawnEmitterAttached` "/Game/VFX_Toolkit_V1/ParticleSystems/356Days/Par_MuzzleFlash1_01.Par_MuzzleFlash1_01" (`self.SkeletalMesh`) "WeaponMuzzle" (0.0 0.0 0.0) (struct) (0.4 0.4 0.4) "SnapToTarget" :!label _label)
  (`GameplayStatics.PlaySound2D` (`self.ShootSound`) 1.0 1.0 0.0 null null)
  (bind _outhit (`KismetSystemLibrary.LineTraceSingle` :`Start` _returnvalue :`End` (select `bool` (`/Game/ThirdPerson/Blueprints/BP_ThirdPersonCharacter.B_InFixedCam` _as_bp_third_person_character) :`false` (+ _returnvalue (* (`KismetMathLibrary.GetForwardVector` (`PlayerCameraManager.GetCameraRotation` (`GameplayStatics.GetPlayerCameraManager` 0))) 10000.0)) :`true` (+ (`self.K2_GetActorLocation` _as_bp_third_person_character) (* (`self.GetActorForwardVector` _as_bp_third_person_character) 10000.0))) :`TraceChannel` "TraceTypeQuery1" :`TraceColor` (struct :`G` 0.570143 :`B` 1.0 :`A` 1.0)))
  (bind (_bblockinghit _binitialoverlap _time _distance _location _impactpoint _normal _impactnormal _physmat _hitactor _hitcomponent _hitbonename _bonename _hititem _elementindex _faceindex _tracestart _traceend) (`GameplayStatics.BreakHitResult` _outhit))
  (bind (_outhit_2 _returnvalue_2) (`KismetSystemLibrary.LineTraceSingle` (`SceneComponent.GetSocketLocation` (`self.SkeletalMesh`) "WeaponMuzzle") (+ _location (* (`KismetMathLibrary.Normal` (- _traceend _tracestart)) 100.0)) "TraceTypeQuery1"))
  (if _returnvalue_2
    (bind (_bblockinghit_2 _binitialoverlap_2 _time_2 _distance_2 _location_2 _impactpoint_2 _normal_2 _impactnormal_2 _physmat_2 _hitactor_2) (`GameplayStatics.BreakHitResult` _outhit_2))
    (if (`KismetSystemLibrary.DoesImplementInterface` _hitactor_2 "/Game/ThirdPerson/Blueprints/Interfaces/INT_BasicEnemy.INT_BasicEnemy_C")
      (message `/Game/ThirdPerson/Blueprints/Interfaces/INT_BasicEnemy.TakeDamage` _hitactor_2 (`self.RangedDamage`)))
    (`GameplayStatics.SpawnEmitterAtLocation` "/Game/VFX_Toolkit_V1/ParticleSystems/356Days/Par_MuzzleFlash1_01.Par_MuzzleFlash1_01" _location_2 (`KismetMathLibrary.MakeRotFromX` _normal_2) (0.5 0.5 0.5))))

(event `CustomEvent`
  ;[1 0.4908 0.3605] Shoot
  (goto _label))

(fn `UserConstructionScript`
  (`parent.UserConstructionScript`))