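; Base Blueprint for ranged weapon pickups that fire hitscan shots at enemies, with damage set on BeginPlay by light or heavy weapon type.
; Shooting spends a bullet, updates the player's ammo widget and plays muzzle flash and sound.
; A trace from the follow camera, aimed along actor forward in fixed-cam mode, guides a second muzzle trace.
; That trace spawns impact effects and damages INT_BasicEnemy actors through the interface.
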(event `self.ReceiveBeginPlay`
  ;[0.2649 1 0.1115] Begin Play
  (`parent.ReceiveBeginPlay`)
  (bind _asbp_third_person_character (cast `/Game/ThirdPerson/Blueprints/BP_ThirdPersonCharacter` (`GameplayStatics.GetPlayerPawn` 0)))
  (set `self.As BP Third Person Character` _asbp_third_person_character)
  (set `self.Strafe Camera` (`/Game/ThirdPerson/Blueprints/BP_ThirdPersonCharacter.FollowCamera` _asbp_third_person_character))
  (set `self.RangedDamage` (select `/Game/PickUpObject/EN_ObjectType` (`self.ObjectType`) :`NewEnumerator2` 30.0 :`NewEnumerator3` 50.0)))

(event `/Game/PickUpObject/RangedWeapons/INT_Weapon.Shoot`
  (bind _as_bp_third_person_character (`self.As BP Third Person Character`))
  (bind _returnvalue (`SceneComponent.K2_GetComponentLocation` (`self.Strafe Camera`)))
  (bind _wg_bullets (`/Game/ThirdPerson/Blueprints/BP_ThirdPersonCharacter.WG_Bullets` (`self.As BP Third Person Character`)))
  ;[1 0.4908 0.3605] Shoot
  (if (> (`self.BulletAmt`) 0) :!label _label
    (`GameplayStatics.SpawnEmitterAttached` "/Game/VFX_Toolkit_V1/ParticleSystems/356Days/Par_MuzzleFlash1_01.Par_MuzzleFlash1_01" (`self.SkeletalMesh`) "WeaponMuzzle" (0.0 0.0 0.0) (struct) (0.4 0.4 0.4) "SnapToTarget")
    (bind _result (`/Engine/EditorBlueprintResources/StandardMacros.DecrementInt` (`self.BulletAmt`))
      (:`  `
        (set `TextBlock.Text` (`KismetTextLibrary.Conv_IntToText` _result) (`/Game/ThirdPerson/Blueprints/HUD/WG_Bullets.TextBlock_0` _wg_bullets))
        (`UserWidget.PlayAnimation` _wg_bullets (`/Game/ThirdPerson/Blueprints/HUD/WG_Bullets.ChangeText` _wg_bullets) 0.0 1 "Forward" 1.0 false)
        (`GameplayStatics.PlaySound2D` (`self.ShootSound`) 1.0 1.0 0.0 null null)
        (bind _outhit (`KismetSystemLibrary.LineTraceSingle` :`Start` _returnvalue :`End` (select `bool` (`/Game/ThirdPerson/Blueprints/BP_ThirdPersonCharacter.B_InFixedCam` _as_bp_third_person_character) :`false` (+ _returnvalue (* (`KismetMathLibrary.GetForwardVector` (`PlayerCameraManager.GetCameraRotation` (`GameplayStatics.GetPlayerCameraManager` 0))) 10000.0)) :`true` (+ (`self.K2_GetActorLocation` _as_bp_third_person_character) (* (`self.GetActorForwardVector` _as_bp_third_person_character) 10000.0))) :`TraceChannel` "TraceTypeQuery1" :`TraceColor` (struct :`G` 0.570143 :`B` 1.0 :`A` 1.0)))
        (bind (_bblockinghit _binitialoverlap _time _distance _location _impactpoint _normal _impactnormal _physmat _hitactor _hitcomponent _hitbonename _bonename _hititem _elementindex _faceindex _tracestart _traceend) (`GameplayStatics.BreakHitResult` _outhit))
        (bind (_outhit_2 _returnvalue_2) (`KismetSystemLibrary.LineTraceSingle` (`SceneComponent.GetSocketLocation` (`self.SkeletalMesh`) "WeaponMuzzle") (+ _location (* (`KismetMathLibrary.Normal` (- _traceend _tracestart)) 100.0)) "TraceTypeQuery1"))
        (if _returnvalue_2
          (bind (_bblockinghit_2 _binitialoverlap_2 _time_2 _distance_2 _location_2 _impactpoint_2 _normal_2 _impactnormal_2 _physmat_2 _hitactor_2) (`GameplayStatics.BreakHitResult` _outhit_2))
          (if (`KismetSystemLibrary.DoesImplementInterface` _hitactor_2 "/Game/ThirdPerson/Blueprints/Interfaces/INT_BasicEnemy.INT_BasicEnemy_C")
            (message `/Game/ThirdPerson/Blueprints/Interfaces/INT_BasicEnemy.TakeDamage` _hitactor_2 (`self.RangedDamage`)))
          (`GameplayStatics.SpawnEmitterAtLocation` "/Game/VFX_Toolkit_V1/ParticleSystems/356Days/Par_MuzzleFlash1_01.Par_MuzzleFlash1_01" _location_2 (`KismetMathLibrary.MakeRotFromX` _normal_2) (0.5 0.5 0.5)))))))

(event `CE_Shoot`
  ;[1 0.4908 0.3605] Shoot
  (goto _label))

(fn `UserConstructionScript`
  (`parent.UserConstructionScript`))