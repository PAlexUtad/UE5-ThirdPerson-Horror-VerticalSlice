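; Generic pickup actor for keys and melee, light or heavy weapons, collected by the player with the interact input.
; The construction script uses the object type to set item class, display mesh (random for melee), transform and key-only spinning.
; Sphere overlap checks eligibility, as one outfit permits only keys.
; Interacting adds keys with optional dialogue, or spawns weapons in free hands, then destroys the pickup.
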(event `self.ReceiveBeginPlay`
  ;[0.008931 1 0.0846] Begin play, rotate mesh if it's a key object
  (`parent.ReceiveBeginPlay`)
  (set `/Game/DialogSystem/DialogComponent.DialogTree` (`self.DialogOnPickUp`) (`self.DialogComponent`))
  (if (`self.DoesRotate`)
    (set `self.RotationDirection` (`KismetMathLibrary.MakeRotator` (`KismetMathLibrary.RandomFloatInRange` -8.0 5.0) (`KismetMathLibrary.RandomFloatInRange` -5.0 8.0) (`KismetMathLibrary.RandomFloatInRange` -10.0 10.0)))
    (`KismetSystemLibrary.K2_SetTimerDelegate` (delegate `RotateDisplayMesh`) 0.1 true)))

(event `RotateDisplayMesh`
  ;[0.008931 1 0.0846] Begin play, rotate mesh if it's a key object
  (`SceneComponent.K2_AddWorldRotation` (`self.StaticMesh`) (`self.RotationDirection`) false false))

(event `self.Sphere.OnComponentBeginOverlap`
  (params (OverlappedComponent :type "PrimitiveComponent Object Reference") (OtherActor :type "Actor Object Reference") (OtherComp :type "PrimitiveComponent Object Reference") (OtherBodyIndex :type Integer) (bFromSweep :type Boolean) (SweepResult :type "HitResult Structure (by ref)"))
  ;[0.3258 0.9035 1] Interaction overlap
  (bind _asbp_third_person_character (cast `/Game/ThirdPerson/Blueprints/BP_ThirdPersonCharacter` OtherActor))
  (bind _output_get (set `self.As BP Third Person Character` _asbp_third_person_character))
  (bind _returnvalue (`self.CanPickUpObject` _output_get))
  (if _returnvalue
    (`self.OnOverlap`)))

(event `self.Sphere.OnComponentEndOverlap`
  (params (OverlappedComponent :type "PrimitiveComponent Object Reference") (OtherActor :type "Actor Object Reference") (OtherComp :type "PrimitiveComponent Object Reference") (OtherBodyIndex :type Integer))
  ;[0.3258 0.9035 1] Interaction overlap
  (if (`KismetSystemLibrary.DoesImplementInterface` OtherActor "/Game/ThirdPerson/Blueprints/Interfaces/BPINT_Player.BPINT_Player_C")
    (set `self.As BP Third Person Character` null)
    (`self.OffOverlap`)))

(event `EnhancedInput|/Game/ThirdPerson/Input/Actions/IA_Interact`
  (params (ActionValue :type Boolean) (ElapsedSeconds :type "Float (double-precision)") (TriggeredSeconds :type "Float (double-precision)") (InputAction :type "InputAction Object Reference" :default "/Game/ThirdPerson/Input/Actions/IA_Interact.IA_Interact"))
  (bind _as_bp_third_person_character (`self.As BP Third Person Character`))
  (bind _as_bp_third_person_character_2 (`self.As BP Third Person Character`))
  (bind _dialogcomponent (`self.DialogComponent`))
  ;[1 0.7142 0.7375] Pick up object, play dialogue if any.
  (:`Triggered`
    (if (`self.CanInt`)
      (set `self.CanInt` false)
      (`/Engine/EditorBlueprintResources/StandardMacros.IsValid` _as_bp_third_person_character
        (:`Is Valid`
          (switch `/Game/PickUpObject/EN_ObjectType` (`self.ObjectType`)
            (:`NewEnumerator1`
              (`/Game/ThirdPerson/Blueprints/BP_ThirdPersonCharacter.Add_Key` _as_bp_third_person_character (`self.BP_ObjectInHand`))
              (if (`KismetSystemLibrary.IsValid` (`/Game/DialogSystem/DialogComponent.DialogTree` _dialogcomponent))
                (set `/Game/ThirdPerson/Blueprints/BP_ThirdPersonCharacter.B_CannotMove` true _as_bp_third_person_character_2)
                (`SceneComponent.SetHiddenInGame` (`self.StaticMesh`) true false)
                (`/Game/DialogSystem/InteractionInterface.OnInteraction` _dialogcomponent _as_bp_third_person_character_2)
                (set `/Game/ThirdPerson/Blueprints/BP_ThirdPersonCharacter.B_CannotMove` false _as_bp_third_person_character_2)
                (`KismetSystemLibrary.Delay` 2.0)
                (`/Game/DialogSystem/DialogComponent.OnExit_Event_0` _dialogcomponent :!label _label))
              (`self.K2_DestroyActor`))
            (:`NewEnumerator0`
              (bind _returnvalue (`/Game/ThirdPerson/Blueprints/BP_ThirdPersonCharacter.IsHoldingObject` _as_bp_third_person_character :!label _label_2))
              (if _returnvalue
                (set `self.CanInt` true)
                (else
                  (set `/Game/ThirdPerson/Blueprints/BP_ThirdPersonCharacter.BP_$ObjectInHand` (`self.BP_ObjectInHand`) _as_bp_third_person_character)
                  (`/Game/ThirdPerson/Blueprints/BP_ThirdPersonCharacter.SpawnObjectPickedUp` _as_bp_third_person_character)
                  (`GameplayStatics.PlaySound2D` "/Game/SFX/SC_PickUpObject.SC_PickUpObject" 1.0 1.0 0.0 null null)
                  (`self.K2_DestroyActor`))))
            (:`NewEnumerator2`
              (goto _label_2))
            (:`NewEnumerator3`
              (goto _label_2))))))))

(event `Key|Gamepad_FaceButton_Bottom`
  (params (Key :type "Key Structure"))
  ;[1 0.7142 0.7375] Pick up object, play dialogue if any.
  (:`Pressed`
    (if (not (`self.CanInt`)) :!label _label_3
      (goto _label))))

(event `EnhancedInput|/Game/ThirdPerson/Input/Actions/IA_Interact`
  (params (ActionValue :type Boolean) (ElapsedSeconds :type "Float (double-precision)") (TriggeredSeconds :type "Float (double-precision)") (InputAction :type "InputAction Object Reference" :default "/Game/ThirdPerson/Input/Actions/IA_Interact.IA_Interact"))
  ;[1 0.7142 0.7375] Pick up object, play dialogue if any.
  (:`Started`
    (goto _label_3)))

(fn `CanPickUpObject`
  (params (PlayerRef :type "/Game/ThirdPerson/Blueprints/BP_ThirdPersonCharacter Object Reference"))
  (returns (ReturnValue :type Boolean))
  (bind _u_currentoutfit_index (`/Game/ThirdPerson/Blueprints/BP_ThirdPersonCharacter.U_CurrentOutfit_Index` PlayerRef))
  ;[1 1 1] Either not wearing the secret costume or is wearing it and can only pick up keys
  (return (or (!= _u_currentoutfit_index 3) (and (== _u_currentoutfit_index 3) (select `/Game/PickUpObject/EN_ObjectType` (`self.ObjectType`) :`NewEnumerator1` true)))))

(fn `UserConstructionScript`
  (bind _returnvalue (`KismetMathLibrary.RandomFloatInRange` -180.0 180.0))
  (bind _objecttype (`self.ObjectType`))
  (bind _staticmesh (`self.StaticMesh`))
  ;[1 1 1] Set Mesh, position and rotation based on the ENUM object type, the mesh can still be overriden if necessary (should do the same with pos, rot and scale tbh)
  (`SphereComponent.SetSphereRadius` (`self.Sphere`) (`self.CollisionRadius`) true)
  (`SceneComponent.SetWorldScale3D` (`self.StaticMesh`) (`self.DisplayMesh_Scale`))
  (set `self.BP_ObjectInHand` (select `/Game/PickUpObject/EN_ObjectType` _objecttype :`NewEnumerator1` (`self.BP_ObjectInHand`) :`NewEnumerator0` "/Game/PickUpObject/BP_Weapon.BP_Weapon_C" :`NewEnumerator2` "/Game/PickUpObject/RangedWeapons/BP_BaseRangedWeapon.BP_BaseRangedWeapon_C" :`NewEnumerator3` "/Game/PickUpObject/RangedWeapons/BP_Rifle.BP_Rifle_C"))
  (bind _output_get (set `self.SM_DisplayMesh` (select `/Game/PickUpObject/EN_ObjectType` _objecttype :`NewEnumerator1` "/Game/Environment/Library/SM_KeyPickUpObj.SM_KeyPickUpObj" :`NewEnumerator0` (select `int` (`KismetMathLibrary.RandomIntegerInRange` 0 3) :`0` "/Game/PickUpObject/MeleeObjects/SM_Weapons_Cube_001.SM_Weapons_Cube_001" :`1` "/Game/PickUpObject/MeleeObjects/SM_Weapons_Cube_002.SM_Weapons_Cube_002" :`2` "/Game/PickUpObject/MeleeObjects/SM_Weapons_Cube_003.SM_Weapons_Cube_003" :`3` "/Game/PickUpObject/MeleeObjects/SM_Weapons_Cube_004.SM_Weapons_Cube_004" :!type "StaticMesh Object Reference") :`NewEnumerator2` "/Game/PickUpObject/RangedWeapons/SM_Gun.SM_Gun" :`NewEnumerator3` "/Game/PickUpObject/RangedWeapons/SM_Rifle.SM_Rifle")))
  (set `self.DoesRotate` (select `/Game/PickUpObject/EN_ObjectType` _objecttype :`NewEnumerator1` true))
  (`StaticMeshComponent.SetStaticMesh` _staticmesh _output_get)
  (`SceneComponent.K2_SetRelativeTransform` _staticmesh (select `/Game/PickUpObject/EN_ObjectType` _objecttype :`NewEnumerator1` (`KismetMathLibrary.MakeTransform` (0.0 0.0 50.0) (struct) (0.5 0.5 0.5)) :`NewEnumerator0` (`KismetMathLibrary.MakeTransform` (0.0 0.0 0.0) (`KismetMathLibrary.MakeRotator` 90.0 0.0 _returnvalue) (0.8 0.8 0.8)) :`NewEnumerator2` (`KismetMathLibrary.MakeTransform` (0.0 0.0 0.0) (`KismetMathLibrary.MakeRotator` 0.0 90.0 _returnvalue)) :`NewEnumerator3` (`KismetMathLibrary.MakeTransform` (0.0 0.0 0.0) (`KismetMathLibrary.MakeRotator` 0.0 90.0 _returnvalue)) :!type "Transform Structure") false false))