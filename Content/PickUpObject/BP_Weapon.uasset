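; Weapon actor in the pickup object set that spins and shows a trail while flying fast.
; BeginPlay runs the parent logic, zeroes projectile velocity, picks one of four cube weapon meshes at random and hides the trail.
; A fast looping timer, used in place of Tick, checks projectile speed.
; Above a speed threshold it reveals the trail and pitches the mesh in proportion to speed, otherwise it hides the trail.
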(event `self.ReceiveBeginPlay`
  (`parent.ReceiveBeginPlay`)
  (set `MovementComponent.Velocity` (0.0 0.0 0.0) (`self.ProjectileMovement`))
  (`StaticMeshComponent.SetStaticMesh` (`self.StaticMesh`) (select `int` (`KismetMathLibrary.RandomIntegerInRange` 0 3) :`0` "/Game/PickUpObject/MeleeObjects/SM_Weapons_Cube_001.SM_Weapons_Cube_001" :`1` "/Game/PickUpObject/MeleeObjects/SM_Weapons_Cube_002.SM_Weapons_Cube_002" :`2` "/Game/PickUpObject/MeleeObjects/SM_Weapons_Cube_003.SM_Weapons_Cube_003" :`3` "/Game/PickUpObject/MeleeObjects/SM_Weapons_Cube_004.SM_Weapons_Cube_004" :!type "StaticMesh Object Reference"))
  (`KismetSystemLibrary.K2_SetTimerDelegate` (delegate `CE_RotateInFlight`) 0.01 true true)
  (`SceneComponent.SetHiddenInGame` (`self.WeaponTrailTurn`) true true))

(event `CE_RotateInFlight`
  (bind _returnvalue (`KismetMathLibrary.VSize` (`MovementComponent.Velocity` (`self.ProjectileMovement`))))
  (if (> _returnvalue 1000.0)
    (`SceneComponent.SetHiddenInGame` (`self.WeaponTrailTurn`) false true)
    (`SceneComponent.K2_AddLocalRotation` (`self.StaticMesh`) (`KismetMathLibrary.MakeRotator` 0.0 (/ _returnvalue 20.0)) false false)
    (else
      (`SceneComponent.SetHiddenInGame` (`self.WeaponTrailTurn`) true true))))

(fn `UserConstructionScript`
  (`parent.UserConstructionScript`))