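; Fixed camera volume that blends the player's view to its own camera while the third-person character is inside.
; Entering the box flags the character, records the camera rotation as its control rotation and adds this actor to the character's overlap list.
; Leaving the box, or an optional outer box, removes it, restoring the character's view only when the list is empty.
; The construction script sizes both boxes from variables.
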(event `self.ReceiveBeginPlay`
  ;[0.4218 1 0.1914] Begin Play
  (bind _asbp_third_person_character (cast `/Game/ThirdPerson/Blueprints/BP_ThirdPersonCharacter` (`GameplayStatics.GetPlayerPawn` 0)))
  (set `self.As BP Third Person Character` _asbp_third_person_character))

(event `self.Box.OnComponentBeginOverlap`
  (params (OverlappedComponent :type "PrimitiveComponent Object Reference") (OtherActor :type "Actor Object Reference") (OtherComp :type "PrimitiveComponent Object Reference") (OtherBodyIndex :type Integer) (bFromSweep :type Boolean) (SweepResult :type "HitResult Structure (by ref)"))
  (bind _as_bp_third_person_character (`self.As BP Third Person Character`))
  ;[1 0.6172 0.3183] Change camera and check if you're still in another fixed cam volume upon ending overlap
  (if (`KismetSystemLibrary.DoesImplementInterface` OtherActor "/Game/ThirdPerson/Blueprints/Interfaces/BPINT_Player.BPINT_Player_C")
    (set `/Game/ThirdPerson/Blueprints/BP_ThirdPersonCharacter.B_InFixedCam` true _as_bp_third_person_character)
    (`KismetArrayLibrary.Array_Append` (`/Game/ThirdPerson/Blueprints/BP_ThirdPersonCharacter.L_FixedCamActorsOvr` _as_bp_third_person_character) (`|MakeArray` self :!type "/Game/FixedCamera/BP_FixedCamera Object Reference"))
    (set `/Game/ThirdPerson/Blueprints/BP_ThirdPersonCharacter.R_FixedControlRot` (`SceneComponent.K2_GetComponentRotation` (`self.Camera`)) _as_bp_third_person_character)
    (`PlayerController.SetViewTargetWithBlend` (`GameplayStatics.GetPlayerController` 0) self (`self.F_blendtime`) "VTBlend_Cubic" 0.0 false)))

(event `self.OutBox.OnComponentEndOverlap`
  (params (OverlappedComponent :type "PrimitiveComponent Object Reference") (OtherActor :type "Actor Object Reference") (OtherComp :type "PrimitiveComponent Object Reference") (OtherBodyIndex :type Integer))
  (bind _as_bp_third_person_character (`self.As BP Third Person Character`))
  (bind _l_fixedcamactorsovr (`/Game/ThirdPerson/Blueprints/BP_ThirdPersonCharacter.L_FixedCamActorsOvr` _as_bp_third_person_character))
  ;[1 0.6172 0.3183] Change camera and check if you're still in another fixed cam volume upon ending overlap
  (if (and (`self.B_UseOutColl`) (`KismetSystemLibrary.DoesImplementInterface` OtherActor "/Game/ThirdPerson/Blueprints/Interfaces/BPINT_Player.BPINT_Player_C"))
    (`KismetArrayLibrary.Array_RemoveItem` _l_fixedcamactorsovr self :!label _label)
    (if (== (`KismetArrayLibrary.Array_Length` _l_fixedcamactorsovr) 0)
      (`PlayerController.SetViewTargetWithBlend` (`GameplayStatics.GetPlayerController` 0) _as_bp_third_person_character (`self.F_blendtime`) "VTBlend_Cubic" 0.0 false)
      (set `/Game/ThirdPerson/Blueprints/BP_ThirdPersonCharacter.B_InFixedCam` false _as_bp_third_person_character)
      (set `/Game/ThirdPerson/Blueprints/BP_ThirdPersonCharacter.R_FixedControlRot` (struct) _as_bp_third_person_character))))

(event `self.Box.OnComponentEndOverlap`
  (params (OverlappedComponent :type "PrimitiveComponent Object Reference") (OtherActor :type "Actor Object Reference") (OtherComp :type "PrimitiveComponent Object Reference") (OtherBodyIndex :type Integer))
  ;[1 0.6172 0.3183] Change camera and check if you're still in another fixed cam volume upon ending overlap
  (if (and (not (`self.B_UseOutColl`)) (`KismetSystemLibrary.DoesImplementInterface` OtherActor "/Game/ThirdPerson/Blueprints/Interfaces/BPINT_Player.BPINT_Player_C"))
    (goto _label)))

(fn `UserConstructionScript`
  (`BoxComponent.SetBoxExtent` (`self.Box`) (`self.V_Coll_Size`) true)
  (`BoxComponent.SetBoxExtent` (`self.OutBox`) (`self.V_Coll_Size_Out`) true))