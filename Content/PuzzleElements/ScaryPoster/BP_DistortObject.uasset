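; BP_DistortObject is a scary poster puzzle element that distorts the screen and plays static as the player approaches.
; When a BPINT_Player actor enters the Box, it stores the entry distance and starts a self-calling Delay loop.
; Each pass fires two 2D static sounds and sets the PC_Pixel collection's "Switch" parameter by closeness relative to entry.
; Leaving the Box clears the player, ending the loop and zeroing the parameter.
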(event `self.Box.OnComponentBeginOverlap`
  (params (OverlappedComponent :type "PrimitiveComponent Object Reference") (OtherActor :type "Actor Object Reference") (OtherComp :type "PrimitiveComponent Object Reference") (OtherBodyIndex :type Integer) (bFromSweep :type Boolean) (SweepResult :type "HitResult Structure (by ref)"))
  ;[0.3395 1 0.5117] Start distortion check on overlap
  (if (`KismetSystemLibrary.DoesImplementInterface` OtherActor "/Game/ThirdPerson/Blueprints/Interfaces/BPINT_Player.BPINT_Player_C")
    (set `self.BP_Player` OtherActor)
    (set `self.F_MaxDistance` (`self.GetDistanceTo` OtherActor self))
    (`self.Distort`)))

(event `Distort`
  (bind _bp_player (`self.BP_Player`))
  (bind _f_maxdistance (`self.F_MaxDistance`))
  ;[1 0.2925 0.1626] Increase post process material parameter based on distance from the player, stop on the end overlap
  (`/Engine/EditorBlueprintResources/StandardMacros.IsValid` _bp_player
    (:`Is Valid`
      (`GameplayStatics.PlaySound2D` "/Game/SFX/WAV/Static/Static.Static" 1.0 1.0 0.0 null null)
      (`GameplayStatics.PlaySound2D` "/Game/SFX/WAV/Static/Static2.Static2" 1.0 1.0 0.0 null null)
      (`KismetMaterialLibrary.SetScalarParameterValue` "/Game/PostProcess/PC_Pixel.PC_Pixel" "Switch" (/ (- _f_maxdistance (`self.GetDistanceTo` _bp_player self)) _f_maxdistance))
      (`KismetSystemLibrary.Delay` 0.05)
      (`self.Distort`))
    (:`Is Not Valid`
      (`KismetMaterialLibrary.SetScalarParameterValue` "/Game/PostProcess/PC_Pixel.PC_Pixel" "Switch" :!label _label))))

(event `self.Box.OnComponentEndOverlap`
  (params (OverlappedComponent :type "PrimitiveComponent Object Reference") (OtherActor :type "Actor Object Reference") (OtherComp :type "PrimitiveComponent Object Reference") (OtherBodyIndex :type Integer))
  ;[1 0.2925 0.1626] Increase post process material parameter based on distance from the player, stop on the end overlap
  (if (`KismetSystemLibrary.DoesImplementInterface` OtherActor "/Game/ThirdPerson/Blueprints/Interfaces/BPINT_Player.BPINT_Player_C")
    (set `self.BP_Player` null)
    (goto _label)))

(fn `UserConstructionScript`)