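; BP_CombinationLock is an inspectable combination lock puzzle that can unlock a linked door.
; While inspecting, left/right input cycles the selected dial and moves an arrow indicator, while up/down rotates it in 45-degree timeline-driven steps.
; After each turn, three dial rotations are compared to the configured combination.
; A match exits inspection, unlocks and triggers any linked door, then destroys the lock.
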(event `self.ReceiveBeginPlay`
  ;[0.189 1 0.02787] Begin Play and remove collision from meshes in case there are any
  (`parent.ReceiveBeginPlay`)
  (`PrimitiveComponent.SetCollisionEnabled` (`self.Cube`) "NoCollision")
  (`PrimitiveComponent.SetCollisionEnabled` (`self.Cube2`) "NoCollision")
  (`PrimitiveComponent.SetCollisionEnabled` (`self.Cube3`) "NoCollision")
  (`PrimitiveComponent.SetCollisionEnabled` (`self.Cube1`) "NoCollision")
  (set `self.B_IsGearRotating` false)
  (set `self.WG_Class` "/Game/PuzzleElements/CombinationLock/WG_CombinationControls.WG_CombinationControls_C"))

(event `ChangePiece`
  (params (Add :type Integer))
  (bind _arrowhud (`self.ArrowHud`))
  (bind (_relativelocation_x _relativelocation_y _relativelocation_z) (`KismetMathLibrary.BreakVector` (`SceneComponent.RelativeLocation` _arrowhud)))
  (bind _returnvalue (- (`SceneComponent.GetNumChildrenComponents` (`self.Cube`)) 1))
  (bind _relativelocation_x_2 (`KismetMathLibrary.BreakVector` (`SceneComponent.RelativeLocation` (`SceneComponent.GetChildComponent` (`self.Cube`) (`self.U_SelectedPiece`)))))
  ;[0.3889 0.9967 1] Change focused piece and modify arrow position for the player to see
  (if (not (`self.B_IsGearRotating`))
    (`/Engine/EditorBlueprintResources/StandardMacros.DoOnce` false :!label _label
      (:`Completed`
        (bind _output_get (set `self.U_SelectedPiece` (+ (`self.U_SelectedPiece`) Add)))
        (if (> _output_get _returnvalue)
          (set `self.U_SelectedPiece` 0)
          (elif (< _output_get 0)
            (set `self.U_SelectedPiece` _returnvalue)))
        (`SceneComponent.K2_SetRelativeLocation` _arrowhud (`KismetMathLibrary.MakeVector` _relativelocation_x (/ _relativelocation_x_2 4.5) _relativelocation_z) false false)
        (`GameplayStatics.PlaySound2D` "/Game/SFX/WAV/Interactions/PickItem3.PickItem3" 1.0 1.0 0.0 null null)))))

(event `EnhancedInput|/Game/ThirdPerson/Input/Actions/IA_SLO_Right`
  (params (ActionValue :type Boolean) (ElapsedSeconds :type "Float (double-precision)") (TriggeredSeconds :type "Float (double-precision)") (InputAction :type "InputAction Object Reference" :default "/Game/ThirdPerson/Input/Actions/IA_SLO_Right.IA_SLO_Right"))
  ;[0.3889 0.9967 1] Change focused piece and modify arrow position for the player to see
  ;;[1 1 1] Use specific actions because this is for lock on stuff and will break everything
  (:`Started`
    (`self.ChangePiece` 1))
  (:`Completed`
    (goto _label :!via `Reset`)))

(event `EnhancedInput|/Game/ThirdPerson/Input/Actions/IA_SLO_Left`
  (params (ActionValue :type Boolean) (ElapsedSeconds :type "Float (double-precision)") (TriggeredSeconds :type "Float (double-precision)") (InputAction :type "InputAction Object Reference" :default "/Game/ThirdPerson/Input/Actions/IA_SLO_Left.IA_SLO_Left"))
  ;[0.3889 0.9967 1] Change focused piece and modify arrow position for the player to see
  (:`Started`
    (`self.ChangePiece` -1))
  (:`Completed`
    (goto _label :!via `Reset`)))

(event `EnhancedInput|/Game/ThirdPerson/Input/Actions/IA_CombLockMoveDown`
  (params (ActionValue :type Boolean) (ElapsedSeconds :type "Float (double-precision)") (TriggeredSeconds :type "Float (double-precision)") (InputAction :type "InputAction Object Reference" :default "/Game/ThirdPerson/Input/Actions/IA_CombLockMoveDown.IA_CombLockMoveDown"))
  (bind (_r_relative_rotation_roll _r_relative_rotation_pitch _r_relative_rotation_yaw) (`KismetMathLibrary.BreakRotator` (`self.R_Relative Rotation`)))
  ;[1 0.9473 0.5916] Rotate piece and check combination
  (:`Started`
    (set `self.F_RotationAmount` 45.0)
    (if (not (`self.B_IsGearRotating`)) :!label _label_2
      (`/Engine/EditorBlueprintResources/StandardMacros.DoOnce` false :!label _label_3
        (:`Completed`
          (`GameplayStatics.PlaySound2D` "/Game/SFX/WAV/Interactions/Button.Button" 1.0 1.0 0.0 null null)
          (set `self.R_Relative Rotation` (`SceneComponent.RelativeRotation` (`SceneComponent.GetChildComponent` (`self.Cube`) (`self.U_SelectedPiece`))))
          (bind (_direction _newtrack_0) (`Timeline|Rotate Piece` :!via `PlayFromStart`)
            (:`Update`
              (`SceneComponent.K2_SetRelativeRotation` (`SceneComponent.GetChildComponent` (`self.Cube`) (`self.U_SelectedPiece`)) (`KismetMathLibrary.RLerp` (`self.R_Relative Rotation`) (`KismetMathLibrary.MakeRotator` (+ _r_relative_rotation_roll (`self.F_RotationAmount`)) _r_relative_rotation_pitch _r_relative_rotation_yaw) _newtrack_0 true) false false)
              (set `self.B_IsGearRotating` true))
            (:`Finished`
              (set `self.B_IsGearRotating` false)
              (`self.CheckCombination`)))))))
  (:`Completed`
    (goto _label_3 :!via `Reset`)))

(event `EnhancedInput|/Game/ThirdPerson/Input/Actions/IA_CombLockMoveUp`
  (params (ActionValue :type Boolean) (ElapsedSeconds :type "Float (double-precision)") (TriggeredSeconds :type "Float (double-precision)") (InputAction :type "InputAction Object Reference" :default "/Game/ThirdPerson/Input/Actions/IA_CombLockMoveUp.IA_CombLockMoveUp"))
  ;[1 0.9473 0.5916] Rotate piece and check combination
  (:`Started`
    (set `self.F_RotationAmount` -45.0)
    (goto _label_2))
  (:`Completed`
    (goto _label_3 :!via `Reset`)))

(event `InputAxisKey|MouseX`
  (params (AxisValue :type "Float (single-precision)")))

(event `CheckCombination`
  (bind _bp_lockeddoor (`self.BP_LockedDoor`))
  (bind _l_correctcombination (`self.L_CorrectCombination`))
  ;[1 0.9473 0.5916] Rotate piece and check combination
  (if (and (== (`SceneComponent.RelativeRotation` (`self.Cube1`)) (`KismetMathLibrary.MakeRotator` (* (- (`|GetArrayItem` _l_correctcombination) 1) 45)) :`ErrorTolerance` 0.1) (== (`SceneComponent.RelativeRotation` (`self.Cube2`)) (`KismetMathLibrary.MakeRotator` (* (- (`|GetArrayItem` _l_correctcombination 1) 1) 45)) :`ErrorTolerance` 0.1) (== (`SceneComponent.RelativeRotation` (`self.Cube3`)) (`KismetMathLibrary.MakeRotator` (* (- (`|GetArrayItem` _l_correctcombination 2) 1) 45)) :`ErrorTolerance` 0.1))
    (set `self.B_Unlocked` true)
    (`/Engine/EditorBlueprintResources/StandardMacros.IsValid` _bp_lockeddoor
      (:`Is Valid`
        (set `/Game/Environment/Appartment/BP_Door.Locked` false _bp_lockeddoor)
        (`self.OffInspect`)
        (set `self.B_CanBeInteracted` false)
        (`self.OnOverlap` (`self.BP_LockedDoor`))
        (`KismetSystemLibrary.Delay` 1.0)
        (`self.K2_DestroyActor`))
      (:`Is Not Valid`
        (`self.OffInspect`)
        (`self.K2_DestroyActor`)))))

(event `InputAxisKey|MouseY`
  (params (AxisValue :type "Float (single-precision)")))

(event `self.OnOverlap`
  ;[0.6242 0.801 1] Whatever this is
  (if (not (`self.B_Unlocked`))
    (`parent.OnOverlap`)))

(event `self.OnInspect`
  ;[1 0.5165 0.3793] Hide/Unhide arrow HUD
  (`parent.OnInspect`)
  (`SceneComponent.SetHiddenInGame` (`self.ArrowHud`) false false))

(event `self.OffInspect`
  ;[1 0.5165 0.3793] Hide/Unhide arrow HUD
  (`parent.OffInspect`)
  (`SceneComponent.SetHiddenInGame` (`self.ArrowHud`) true false))

(fn `UserConstructionScript`
  (`SphereComponent.SetSphereRadius` (`self.Sphere`) (`self.CollisionRadius`) true))