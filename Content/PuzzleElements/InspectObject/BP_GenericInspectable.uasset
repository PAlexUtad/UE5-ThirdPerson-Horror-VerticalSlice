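; Base inspectable puzzle object that the player can examine up close, with mesh and material set in the construction script.
; Interacting toggles inspection: it locks and hides the player, blends the view to this actor, lifts the mesh to an Arrow via timeline and shows a controls widget.
; While Inspect is held, mouse or move input rotates the mesh.
; Leaving restores the player, camera and initial mesh transform.
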(event `self.ReceiveBeginPlay`
  (bind _cube (`self.Cube`))
  ;[0.2297 1 0.03922] BeginPlay
  (`parent.ReceiveBeginPlay`)
  (set `self.WG_Class` "/Game/PuzzleElements/InspectObject/WG_InspectControls.WG_InspectControls_C")
  (set `self.R_InitialRotation` (`SceneComponent.K2_GetComponentRotation` _cube))
  (set `self.V_InitialLocation` (`SceneComponent.K2_GetComponentLocation` _cube))
  (bind _asbp_third_person_character (cast `/Game/ThirdPerson/Blueprints/BP_ThirdPersonCharacter` (`GameplayStatics.GetPlayerPawn` 0)))
  (set `self.As BP Third Person Character` _asbp_third_person_character))

(event `MoveStaticMesh`
  ;[0.4305 0.9967 1] Move when interacted with, to the world position of the arrow (so that it is in the air and not colliding with environment props)
  (bind (_direction _float) (`Timeline|Timeline` :!label _label)
    (:`Update`
      (`SceneComponent.K2_SetWorldLocation` (`self.Cube`) (`KismetMathLibrary.VLerp` (`self.V_InitialLocation`) (`SceneComponent.K2_GetComponentLocation` (`self.Arrow`)) _float) false false))))

(event `ReInitStaticMesh`
  ;[0.4305 0.9967 1] Move when interacted with, to the world position of the arrow (so that it is in the air and not colliding with environment props)
  (goto _label :!via `Reverse`))

(event `EnhancedInput|/Game/ThirdPerson/Input/Actions/IA_Inspect`
  (params (ActionValue :type Boolean) (ElapsedSeconds :type "Float (double-precision)") (TriggeredSeconds :type "Float (double-precision)") (InputAction :type "InputAction Object Reference" :default "/Game/ThirdPerson/Input/Actions/IA_Inspect.IA_Inspect"))
  ;[1 0.4621 0.3251] Inputs
  (:`Started`
    (set `self.B_IsRotating` true))
  (:`Canceled`
    (set `self.B_IsRotating` false :!label _label_2))
  (:`Completed`
    (goto _label_2)))

(event `InputAxisKey|MouseX`
  (params (AxisValue :type "Float (single-precision)"))
  ;[1 0.4621 0.3251] Inputs
  ;;[1 1 1] Make a single func or smthg idk the code police will kill me
  (if (`self.B_IsRotating`)
    (`SceneComponent.K2_SetWorldRotation` (`self.Cube`) (`KismetMathLibrary.ComposeRotators` (`SceneComponent.K2_GetComponentRotation` (`self.Cube`)) (`KismetMathLibrary.MakeRotator` 0.0 0.0 (* AxisValue (`self.F_RotSpeed`)))) false false)))

(event `EnhancedInput|/Game/ThirdPerson/Input/Actions/IA_Move`
  (params (ActionValue :type "Vector2D Structure") (ElapsedSeconds :type "Float (double-precision)") (TriggeredSeconds :type "Float (double-precision)") (InputAction :type "InputAction Object Reference" :default "/Game/ThirdPerson/Input/Actions/IA_Move.IA_Move"))
  (bind _f_rotspeedcontroller (`self.F_RotSpeedController`))
  ;[1 0.4621 0.3251] Inputs
  ;;[1 1 1] Make a single func or smthg idk the code police will kill me
  (:`Triggered`
    (if (`self.B_IsRotating`)
      (`SceneComponent.K2_SetWorldRotation` (`self.Cube`) (`KismetMathLibrary.ComposeRotators` (`SceneComponent.K2_GetComponentRotation` (`self.Cube`)) (`KismetMathLibrary.MakeRotator` 0.0 (* ActionValue_Y _f_rotspeedcontroller) (* ActionValue_X _f_rotspeedcontroller))) false false))))

(event `InputAxisKey|MouseY`
  (params (AxisValue :type "Float (single-precision)"))
  ;[1 0.4621 0.3251] Inputs
  ;;[1 1 1] Make a single func or smthg idk the code police will kill me
  (if (`self.B_IsRotating`)
    (`SceneComponent.K2_SetWorldRotation` (`self.Cube`) (`KismetMathLibrary.ComposeRotators` (`SceneComponent.K2_GetComponentRotation` (`self.Cube`)) (`KismetMathLibrary.MakeRotator` 0.0 (* AxisValue (`self.F_RotSpeed`)))) false false)))

(event `OnInspect`
  (bind _as_bp_third_person_character (`self.As BP Third Person Character`))
  ;[0.4442 0.4912 1] Interact override, not even sure I need all that
  (set `/Game/ThirdPerson/Blueprints/BP_ThirdPersonCharacter.B_CannotMove` true _as_bp_third_person_character)
  (`/Game/ThirdPerson/Blueprints/BP_ThirdPersonCharacter.StopLockOn` _as_bp_third_person_character)
  (`PlayerController.SetViewTargetWithBlend` (`GameplayStatics.GetPlayerController` 0) self 1.0 "VTBlend_Cubic" 0.0 false)
  (`SceneComponent.SetHiddenInGame` (`self.Widget`) true false)
  (`self.MoveStaticMesh`)
  (`self.SetActorHiddenInGame` (`GameplayStatics.GetPlayerPawn` 0) true)
  (bind _returnvalue (`|CreateWidget` (`self.WG_Class`)))
  (set `self.WG_Controls` _returnvalue)
  (`UserWidget.AddToViewport` (`self.WG_Controls`) 0))

(event `EnhancedInput|/Game/ThirdPerson/Input/Actions/IA_Interact`
  (params (ActionValue :type Boolean) (ElapsedSeconds :type "Float (double-precision)") (TriggeredSeconds :type "Float (double-precision)") (InputAction :type "InputAction Object Reference" :default "/Game/ThirdPerson/Input/Actions/IA_Interact.IA_Interact"))
  ;[0.4442 0.4912 1] Interact override, not even sure I need all that
  (:`Started`
    (if (`self.B_CanBeInteracted`)
      (`/Engine/EditorBlueprintResources/StandardMacros.FlipFlop`
        (:`A`
          (`self.OnInspect`))
        (:`B`
          (`self.OffInspect` :!label _label_3))))))

(event `EnhancedInput|/Game/ThirdPerson/Input/Actions/IA_LeaveInspect`
  (params (ActionValue :type Boolean) (ElapsedSeconds :type "Float (double-precision)") (TriggeredSeconds :type "Float (double-precision)") (InputAction :type "InputAction Object Reference" :default "/Game/ThirdPerson/Input/Actions/IA_LeaveInspect.IA_LeaveInspect"))
  ;[0.4442 0.4912 1] Interact override, not even sure I need all that
  (:`Started`
    (goto _label_3)))

(event `OffInspect`
  (bind _wg_controls (`self.WG_Controls`))
  (bind _as_bp_third_person_character (`self.As BP Third Person Character`))
  ;[0.4442 0.4912 1] Interact override, not even sure I need all that
  (set `/Game/ThirdPerson/Blueprints/BP_ThirdPersonCharacter.B_CannotMove` false _as_bp_third_person_character)
  (`PlayerController.SetViewTargetWithBlend` (`GameplayStatics.GetPlayerController` 0) _as_bp_third_person_character 1.0 "VTBlend_Cubic" 0.0 false)
  (`SceneComponent.K2_SetWorldRotation` (`self.Cube`) (`self.R_InitialRotation`) false false)
  (`self.ReInitStaticMesh`)
  (`self.SetActorHiddenInGame` (`GameplayStatics.GetPlayerPawn` 0) false)
  (`/Engine/EditorBlueprintResources/StandardMacros.IsValid` _wg_controls
    (:`Is Valid`
      (`Widget.RemoveFromParent` _wg_controls))))

(fn `UserConstructionScript`
  (bind _cube (`self.Cube`))
  (`StaticMeshComponent.SetStaticMesh` _cube (`self.SM_InspectMesh`))
  (`SceneComponent.K2_SetRelativeTransform` _cube (`KismetMathLibrary.MakeTransform` (`self.V_InitialLocation`) (`self.R_InitialRotation`) (`self.V_InitialScale`)) false false)
  (`PrimitiveComponent.SetMaterial` _cube 0 (`self.M_Material`)))