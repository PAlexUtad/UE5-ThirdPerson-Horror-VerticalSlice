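; BP_OutfitChecker is a puzzle element that gates a referenced door behind the player's current outfit.
; On BeginPlay it caches the player character, locks the door and binds to the door actor's begin-overlap event.
; An overlap while wearing outfit index 0 freezes the player and starts the NeedWorkOutfit dialogue through the character's DialogComponent; any other outfit unlocks the door.
; The overlap handler does not check which actor triggered it.
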(event `self.ReceiveBeginPlay`
  ;[0.283 1 0.2725] Begin play, bind on overlap event to check the outfit
  (bind _asbp_third_person_character (cast `/Game/ThirdPerson/Blueprints/BP_ThirdPersonCharacter` (`GameplayStatics.GetPlayerPawn` 0)))
  (set `self.As BP Third Person Character` _asbp_third_person_character)
  (set `/Game/Environment/BP_SwitchLevelDoor.B_IsLocked` true (`self.DoorRef`))
  (add `self.OnActorBeginOverlap` (`self.DoorRef`) (delegate `MessageOutfit`)))

(event `MessageOutfit` :!signature `self.OnActorBeginOverlap`
  (params (OverlappedActor :type "Actor Object Reference") (OtherActor :type "Actor Object Reference"))
  (bind _as_bp_third_person_character (`self.As BP Third Person Character`))
  (bind _dialogcomponent (`/Game/ThirdPerson/Blueprints/BP_ThirdPersonCharacter.DialogComponent` _as_bp_third_person_character))
  ;[1 0.6373 0.4718] Open dialogue if outfit is wrong
  (if (== (`/Game/ThirdPerson/Blueprints/BP_ThirdPersonCharacter.U_CurrentOutfit_Index` _as_bp_third_person_character) 0)
    (set `/Game/ThirdPerson/Blueprints/BP_ThirdPersonCharacter.B_CannotMove` true _as_bp_third_person_character)
    (set `/Game/DialogSystem/DialogComponent.DialogTree` "/Game/DialogSystem/DialogTree/DialogTree_NeedWorkOutfit.DialogTree_NeedWorkOutfit" _dialogcomponent)
    (`/Game/DialogSystem/InteractionInterface.OnInteraction` _dialogcomponent _as_bp_third_person_character)
    (else
      (set `/Game/Environment/BP_SwitchLevelDoor.B_IsLocked` false (`self.DoorRef`)))))

(fn `UserConstructionScript`)