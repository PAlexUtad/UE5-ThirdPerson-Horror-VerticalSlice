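; Interactable apartment door that swings open on the interact input and can be locked behind a key object.
; When locked, overlap and interact check the player's obtained keys, and a failed interaction plays a locked sound.
; A dot product picks the swing direction from the player's side, and a timeline rotates the door with mesh collision off while moving.
; Leaving the overlap reverses it after a delay, with a close sound if it was open wide.
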(event `self.ReceiveBeginPlay`
  (`parent.ReceiveBeginPlay`)
  (if (`self.Locked`)
    (bind _asbp_third_person_character (cast `/Game/ThirdPerson/Blueprints/BP_ThirdPersonCharacter` (`GameplayStatics.GetPlayerPawn` 0)))
    (set `self.PlayerRef` _asbp_third_person_character)))

(event `self.OnOverlap`
  (bind _playerref (`self.PlayerRef`))
  (if (`KismetSystemLibrary.IsValid` _playerref)
    (if (or (not (`self.Locked`)) (!= (`KismetArrayLibrary.Array_Find` (`/Game/ThirdPerson/Blueprints/BP_ThirdPersonCharacter.L_Keys_Obtained` _playerref) (`self.KeyObject`)) -1))
      (`parent.OnOverlap` :!label _label))
    (else
      (goto _label))))

(event `self.OffOverlap`
  (bind _sm_door_sm_doorframe_002 (`self.SM_Door_SM_DoorFrame_002`))
  (bind (_relativerotation_roll _relativerotation_pitch _relativerotation_yaw) (`KismetMathLibrary.BreakRotator` (`SceneComponent.RelativeRotation` (`self.Scene`))))
  (`parent.OffOverlap`)
  (`KismetSystemLibrary.Delay` 1.0)
  (set `self.StartingYaw` _relativerotation_yaw)
  (bind (_direction _newtrack_0) (`Timeline|Open` :!via `Reverse` :!label _label_2)
    (:`Update`
      (`SceneComponent.K2_SetRelativeRotation` (`self.Scene`) (`KismetMathLibrary.RLerp` (struct) (`KismetMathLibrary.MakeRotator` 0.0 0.0 (`self.TargetYaw`)) _newtrack_0) false false)
      (`PrimitiveComponent.SetCollisionEnabled` _sm_door_sm_doorframe_002 "NoCollision"))
    (:`Finished`
      (`PrimitiveComponent.SetCollisionEnabled` _sm_door_sm_doorframe_002 "QueryAndPhysics")
      (if (> (`KismetMathLibrary.Abs` (`self.StartingYaw`)) 45.0)
        (`GameplayStatics.PlaySoundAtLocation` "/Game/SFX/SC_DoorClose.SC_DoorClose" (`self.K2_GetActorLocation`) (struct) 1.0 1.0 0.0 null null null null)
        (set `self.StartingYaw` 0.0)))))

(event `EnhancedInput|/Game/ThirdPerson/Input/Actions/IA_Interact`
  (params (ActionValue :type Boolean) (ElapsedSeconds :type "Float (double-precision)") (TriggeredSeconds :type "Float (double-precision)") (InputAction :type "InputAction Object Reference" :default "/Game/ThirdPerson/Input/Actions/IA_Interact.IA_Interact"))
  (:`Started`
    (if (`KismetSystemLibrary.IsValid` (`self.PlayerRef`))
      (if (or (not (`self.Locked`)) (!= (`KismetArrayLibrary.Array_Find` (`/Game/ThirdPerson/Blueprints/BP_ThirdPersonCharacter.L_Keys_Obtained` (`self.PlayerRef`)) (`self.KeyObject`)) -1))
        (if (< (`KismetMathLibrary.Dot_VectorVector` (`SceneComponent.GetForwardVector` (`self.Arrow`)) (`KismetMathLibrary.Normal` (- (`self.K2_GetActorLocation`) (`self.K2_GetActorLocation` (`GameplayStatics.GetPlayerPawn` 0))))) 0.0) :!label _label_3
          (set `self.TargetYaw` -95.0)
          (else
            (set `self.TargetYaw` 95.0)))
        (`GameplayStatics.PlaySoundAtLocation` "/Game/SFX/SC_DoorOpen.SC_DoorOpen" (`self.K2_GetActorLocation`) (struct) 1.0 1.0 0.0 null null null null)
        (goto _label_2)
        (else
          (`GameplayStatics.PlaySoundAtLocation` "/Game/SFX/SC_DoorLocked.SC_DoorLocked" (`self.K2_GetActorLocation`) (struct) 1.0 1.0 0.0 null null null null)))
      (else
        (goto _label_3)))))

(fn `UserConstructionScript`)