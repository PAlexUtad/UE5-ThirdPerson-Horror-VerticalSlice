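; Interactable apartment dresser that opens and closes a 3D overlay widget when the player presses interact.
; Begin Play runs the parent logic, creates the widget and caches the third-person character; the construction script sets the collision radius.
; A FlipFlop on IA_Interact toggles the overlay, movement lock, mouse cursor and input mode, playing door open and close sounds.
; The interact event itself performs no proximity check.
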(event `self.ReceiveBeginPlay`
  ;[0 1 0.01019] Begin Play
  (`parent.ReceiveBeginPlay`)
  (bind _returnvalue (`|CreateWidget` "/Game/3D_Widget/WG_3dOvrlay.WG_3dOvrlay_C"))
  (set `self.3D_Ovrlay` _returnvalue)
  (bind _asbp_third_person_character (cast `/Game/ThirdPerson/Blueprints/BP_ThirdPersonCharacter` (`GameplayStatics.GetPlayerPawn` 0)))
  (set `self.As BP Third Person Character` _asbp_third_person_character))

(event `EnhancedInput|/Game/ThirdPerson/Input/Actions/IA_Interact`
  (params (ActionValue :type Boolean) (ElapsedSeconds :type "Float (double-precision)") (TriggeredSeconds :type "Float (double-precision)") (InputAction :type "InputAction Object Reference" :default "/Game/ThirdPerson/Input/Actions/IA_Interact.IA_Interact"))
  (bind _returnvalue (`GameplayStatics.GetPlayerController` 0))
  (bind _3d_ovrlay (`self.3D_Ovrlay`))
  (bind _as_bp_third_person_character (`self.As BP Third Person Character`))
  ;[1 0.4003 0] On Interaction
  (:`Started`
    (`/Engine/EditorBlueprintResources/StandardMacros.FlipFlop`
      (:`A`
        (`UserWidget.AddToViewport` _3d_ovrlay 0)
        (set `/Game/ThirdPerson/Blueprints/BP_ThirdPersonCharacter.B_CannotMove` true _as_bp_third_person_character)
        (set `PlayerController.bShowMouseCursor` true _returnvalue)
        (`WidgetBlueprintLibrary.SetInputMode_GameAndUIEx` _returnvalue null)
        (`GameplayStatics.PlaySound2D` "/Game/SFX/SC_DoorOpen.SC_DoorOpen" 1.0 1.0 0.0 null null))
      (:`B`
        (`Widget.RemoveFromParent` _3d_ovrlay)
        (set `/Game/ThirdPerson/Blueprints/BP_ThirdPersonCharacter.B_CannotMove` false _as_bp_third_person_character)
        (set `PlayerController.bShowMouseCursor` false _returnvalue)
        (`WidgetBlueprintLibrary.SetInputMode_GameOnly` _returnvalue)
        (`GameplayStatics.PlaySound2D` "/Game/SFX/SC_DoorClose.SC_DoorClose" 1.0 1.0 0.0 null null)))))

(fn `UserConstructionScript`
  (set `self.CollisionRadius` 150.0))