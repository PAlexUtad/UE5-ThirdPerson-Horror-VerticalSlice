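; BP_Lightswitch is an apartment light switch that toggles an assigned set of lights and their fixture meshes off and on.
; BeginPlay caches each valid light's intensity and hides the Widget.
; IA_Interact plays a button sound and flip-flops between TurnOff and TurnOn, starting with off.
; These zero or restore intensities and swap fixture materials at per-asset slots, using optional per-asset "on" materials with an emissive default.
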(event `self.ReceiveBeginPlay`
  ;[0 1 0.08637] Begin Play
  (for _array_element (`self.Light`)
    (`/Engine/EditorBlueprintResources/StandardMacros.IsValid` _array_element
      (:`Is Valid`
        (`KismetArrayLibrary.Array_Add` (`self.BaseIntensity`) (`LightComponentBase.Intensity` (`Light.LightComponent` _array_element))))))
  (`SceneComponent.SetHiddenInGame` (`self.Widget`) true false))

(event `TurnOff`
  ;[0.1681 0.302 0.4149] Turn Off
  (for _array_element (`self.Light`)
    (`/Engine/EditorBlueprintResources/StandardMacros.IsValid` _array_element
      (:`Is Valid`
        (`LightComponent.SetIntensity` (`Light.LightComponent` _array_element) 0.0))))
  (for (_array_element_2 _array_index) (`self.LightAsset`)
    (`PrimitiveComponent.SetMaterial` (`StaticMeshActor.StaticMeshComponent` _array_element_2) (`|GetArrayItem` (`self.MaterialIndex`) _array_index) "/Game/Environment/Materials/MI_EmissiveOFF_Inst.MI_EmissiveOFF_Inst")))

(event `TurnOn`
  ;[1 0.2243 0.3074] TurnOn
  (for (_array_element _array_index) (`self.Light`)
    (`/Engine/EditorBlueprintResources/StandardMacros.IsValid` _array_element
      (:`Is Valid`
        (`LightComponent.SetIntensity` (`Light.LightComponent` _array_element) (`|GetArrayItem` (`self.BaseIntensity`) _array_index)))))
  (for (_array_element_2 _array_index_2) (`self.LightAsset`)
    (bind _output (`|GetArrayItem` (`self.On_Material`) _array_index_2))
    (if (`KismetSystemLibrary.IsValid` _output)
      (bind _staticmeshcomponent (`StaticMeshActor.StaticMeshComponent` _array_element_2))
      (bind _output_2 (`|GetArrayItem` (`self.MaterialIndex`) _array_index_2))
      (`PrimitiveComponent.SetMaterial` _staticmeshcomponent _output_2 _output)
      (else
        (`PrimitiveComponent.SetMaterial` _staticmeshcomponent _output_2 "/Game/Environment/Materials/MI_Emissive_Inst.MI_Emissive_Inst")))))

(event `EnhancedInput|/Game/ThirdPerson/Input/Actions/IA_Interact`
  (params (ActionValue :type Boolean) (ElapsedSeconds :type "Float (double-precision)") (TriggeredSeconds :type "Float (double-precision)") (InputAction :type "InputAction Object Reference" :default "/Game/ThirdPerson/Input/Actions/IA_Interact.IA_Interact"))
  ;[1 0.3252 0] Interact With Switch
  (:`Started`
    (`GameplayStatics.PlaySound2D` "/Game/SFX/WAV/Interactions/Button.Button" 1.0 1.0 0.0 null null)
    (`/Engine/EditorBlueprintResources/StandardMacros.FlipFlop`
      (:`A`
        (`self.TurnOff`))
      (:`B`
        (`self.TurnOn`)))))

(fn `UserConstructionScript`)