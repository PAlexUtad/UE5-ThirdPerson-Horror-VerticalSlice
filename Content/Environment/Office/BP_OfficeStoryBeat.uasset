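; Office story beat interactable that turns the office into a creepy, dark scene when the player interacts.
; The parent overlap logic runs only while the scene is lit and the player holds the generic file key.
; Interaction fades screen and music, then reveals fog, kills point lights, neon and all but one computer screen, and removes NPCs.
; It also re-angles the directional light, restores the hidden AuraEntity to its sitting position and starts ambience.
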(event `self.ReceiveBeginPlay`
  (bind _auraentity (`self.AuraEntity`))
  (`parent.ReceiveBeginPlay`)
  (set `self.SittingPosition` (`self.K2_GetActorLocation` _auraentity))
  (`self.K2_SetActorLocation` _auraentity (100000.0 1000000.0 10000.0) false true))

(event `self.OnOverlap`
  (bind _asbp_third_person_character (cast `/Game/ThirdPerson/Blueprints/BP_ThirdPersonCharacter` (`GameplayStatics.GetPlayerPawn` 0)))
  (if (and (!= (`KismetArrayLibrary.Array_Find` (`/Game/ThirdPerson/Blueprints/BP_ThirdPersonCharacter.L_Keys_Obtained` _asbp_third_person_character) "/Game/PickUpObject/BP_GenericFile.BP_GenericFile_C") -1) (not (`self.B_IsDark`)))
    (`parent.OnOverlap`)))

(event `EnhancedInput|/Game/ThirdPerson/Input/Actions/IA_Interact`
  (params (ActionValue :type Boolean) (ElapsedSeconds :type "Float (double-precision)") (TriggeredSeconds :type "Float (double-precision)") (InputAction :type "InputAction Object Reference" :default "/Game/ThirdPerson/Input/Actions/IA_Interact.IA_Interact"))
  (:`Triggered`
    (if (not (`self.B_IsDark`))
      (bind _returnvalue (`|CreateWidget` "/Game/Environment/WG_Fade.WG_Fade_C" (`GameplayStatics.GetPlayerController` 0)))
      (bind _output_get (set `self.FadeWidget` _returnvalue))
      (`UserWidget.AddToViewport` _output_get 0)
      (`/Game/Environment/WG_Fade.FadeInOut` _output_get)
      (bind _asbp_game_instance (cast `/Game/ThirdPerson/Blueprints/BP_GameInstance` (`GameplayStatics.GetGameInstance`)))
      (`/Game/ThirdPerson/Blueprints/BP_GameInstance.CE_FadeOutMusic` _asbp_game_instance)
      (`KismetSystemLibrary.Delay` 1.0)
      (`self.SetUpCreepyScene`)
      (`/Game/ThirdPerson/Blueprints/BP_GameInstance.CE_PlayLevelMusic` _asbp_game_instance "/Game/Music/FWAmbience/SC_FWAmbience.SC_FWAmbience"))))

(fn `SetUpCreepyScene`
  (`SceneComponent.SetVisibility` (`self.Widget`) false false)
  (set `self.B_IsDark` true)
  (`self.SetActorHiddenInGame` (`self.Fog`) false)
  (bind _outactors (`GameplayStatics.GetAllActorsOfClass` "/Script/Engine.PointLight"))
  (for _array_element _outactors
    (`LightComponent.SetIntensity` (`PointLight.PointLightComponent` _array_element) 0.0))
  (`self.K2_SetActorRotation` (`self.DirectionalLight`) (`KismetMathLibrary.MakeRotator` 376.0 80.0 -64.0) false)
  (bind _outactors_2 (`GameplayStatics.GetAllActorsOfClass` "/Script/Engine.StaticMeshActor"))
  (for _array_element_2 _outactors_2
    (if (`KismetStringLibrary.Contains` (`KismetSystemLibrary.GetDisplayName` _array_element_2) "Neon")
      (`PrimitiveComponent.SetMaterial` (`StaticMeshActor.StaticMeshComponent` _array_element_2) 0 "/Game/Environment/Materials/MI_EmissiveOFF_Inst.MI_EmissiveOFF_Inst")))
  (bind _outactors_3 (`GameplayStatics.GetAllActorsOfClass` "/Game/ThirdPerson/Blueprints/BP_GenericNPC.BP_GenericNPC_C"))
  (for _array_element_3 _outactors_3
    (`self.K2_DestroyActor` _array_element_3))
  (`self.K2_SetActorLocation` (`self.AuraEntity`) (`self.SittingPosition`) false true)
  (bind _outactors_4 (`GameplayStatics.GetAllActorsOfClass` "/Script/Engine.StaticMeshActor"))
  (for _array_element_4 _outactors_4
    (if (and (`KismetStringLibrary.Contains` (`KismetSystemLibrary.GetDisplayName` _array_element_4) "Computer_poly") (!= _array_element_4 (`self.OnComputer`)))
      (`PrimitiveComponent.SetMaterial` (`StaticMeshActor.StaticMeshComponent` _array_element_4) 1 "/Game/Environment/Materials/MI_EmissiveOFF_Inst.MI_EmissiveOFF_Inst"))))

(fn `UserConstructionScript`
  (`parent.UserConstructionScript`))