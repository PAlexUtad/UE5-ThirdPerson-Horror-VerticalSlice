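; A generic base actor for interactables that shows a prompt widget and accepts input while a player is nearby.
; A sphere trigger, sized by CollisionRadius in the construction script, reacts only to actors implementing BPINT_Player.
; Its overlaps call OnOverlap and OffOverlap custom events, which toggle the widget and player 0's input on the actor.
; These events are separate so child Blueprints can alter the flow.
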(event `self.ReceiveBeginPlay`
  ;[0.336 1 0.3225] BeginPlay
  (`SceneComponent.SetHiddenInGame` (`self.Widget`) true false))

(event `self.Sphere.OnComponentBeginOverlap`
  (params (OverlappedComponent :type "PrimitiveComponent Object Reference") (OtherActor :type "Actor Object Reference") (OtherComp :type "PrimitiveComponent Object Reference") (OtherBodyIndex :type Integer) (bFromSweep :type Boolean) (SweepResult :type "HitResult Structure (by ref)"))
  ;[0 0.5431 1] Overlap Events
  (if (`KismetSystemLibrary.DoesImplementInterface` OtherActor "/Game/ThirdPerson/Blueprints/Interfaces/BPINT_Player.BPINT_Player_C")
    (`self.OnOverlap`)))

(event `self.Sphere.OnComponentEndOverlap`
  (params (OverlappedComponent :type "PrimitiveComponent Object Reference") (OtherActor :type "Actor Object Reference") (OtherComp :type "PrimitiveComponent Object Reference") (OtherBodyIndex :type Integer))
  ;[0 0.5431 1] Overlap Events
  (if (`KismetSystemLibrary.DoesImplementInterface` OtherActor "/Game/ThirdPerson/Blueprints/Interfaces/BPINT_Player.BPINT_Player_C")
    (`self.OffOverlap`)))

(event `OnOverlap`
  ;[1 0.3619 0] Custom Events in case the children need to modify flow
  (`self.EnableInput` (`GameplayStatics.GetPlayerController` 0))
  (`SceneComponent.SetHiddenInGame` (`self.Widget`) false false))

(event `OffOverlap`
  ;[1 0.3619 0] Custom Events in case the children need to modify flow
  (`self.DisableInput` (`GameplayStatics.GetPlayerController` 0))
  (`SceneComponent.SetHiddenInGame` (`self.Widget`) true false))

(fn `UserConstructionScript`
  (`SphereComponent.SetSphereRadius` (`self.Sphere`) (`self.CollisionRadius`) true))