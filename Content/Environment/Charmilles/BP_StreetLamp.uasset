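; Street lamp Blueprint that switches its spot light and emissive material on or off according to the pitch of a referenced light actor.
; From BeginPlay, CheckDayTime turns the lamp on when pitch is above a fixed threshold and off otherwise.
; It repeats itself after a short random delay rather than using Tick.
; Without a valid LightActor, it only sets the emissive material and never polls.
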(event `self.ReceiveBeginPlay`
  (`/Engine/EditorBlueprintResources/StandardMacros.IsValid` (`self.LightActor`)
    (:`Is Valid`
      (`self.CheckDayTime`))
    (:`Is Not Valid`
      (`PrimitiveComponent.SetMaterial` (`self.SM_CityProps_Cube_012`) 1 "/Game/Environment/Materials/MI_Emissive_Inst.MI_Emissive_Inst"))))

(event `CheckDayTime`
  (bind _sm_cityprops_cube_012 (`self.SM_CityProps_Cube_012`))
  (bind _spotlight (`self.SpotLight`))
  (bind (_returnvalue_roll _returnvalue_pitch) (`KismetMathLibrary.BreakRotator` (`self.K2_GetActorRotation` (`self.LightActor`))))
  (if (> _returnvalue_pitch -6.0)
    (`LightComponent.SetIntensity` _spotlight (`self.OnIntensity`))
    (`PrimitiveComponent.SetMaterial` _sm_cityprops_cube_012 1 "/Game/Environment/Materials/MI_Emissive_Inst.MI_Emissive_Inst")
    (else
      (`LightComponent.SetIntensity` _spotlight 0.0)
      (`PrimitiveComponent.SetMaterial` _sm_cityprops_cube_012 1 "/Game/Environment/Materials/MI_EmissiveOFF_Inst.MI_EmissiveOFF_Inst")))
  (`KismetSystemLibrary.Delay` (`KismetMathLibrary.RandomFloatInRange` 2.0 3.0))
  (`self.CheckDayTime`))

(fn `UserConstructionScript`)