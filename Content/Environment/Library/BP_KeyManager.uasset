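; Library key manager that spawns key pickups at random key locations, with the first two being duds and the third the real key.
; BeginPlay gathers every BP_KeyLocation actor in the level.
; SpawnKey shuffles those locations, spawns a rotating BP_Generic_PickUp with the matching in-hand object and dialog, then removes the used location.
; A still-valid previous key blocks spawning only while the counter is below three.
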(event `self.ReceiveBeginPlay`
  (bind _outactors (`GameplayStatics.GetAllActorsOfClass` "/Game/Environment/Library/BP_KeyLocation.BP_KeyLocation_C"))
  (set `self.KeyLocations` _outactors))

(event `SpawnKey`
  (bind _keylocations (`self.KeyLocations`))
  (bind _output (`|GetArrayItem` _keylocations))
  (bind _returnvalue (< (`self.KeyCounter`) 3))
  (if (not (and (`KismetSystemLibrary.IsValid` (`self.SpawnedKey`)) (< (`self.KeyCounter`) 3)))
    (`KismetArrayLibrary.Array_Shuffle` _keylocations)
    (`/Engine/EditorBlueprintResources/StandardMacros.IncrementInt` (`self.KeyCounter`)
      (:`  `
        (bind _returnvalue_2 (`|SpawnActorFromClass` "/Game/PickUpObject/BP_Generic_PickUp.BP_Generic_PickUp_C" (`KismetMathLibrary.MakeTransform` (`self.K2_GetActorLocation` _output)) "Undefined" "MultiplyWithRoot" null 100.0 "/Game/Environment/Library/SM_KeyPickUpObj.SM_KeyPickUpObj" (0.5 0.5 0.5) (select `bool` _returnvalue :`false` "/Game/PickUpObject/BP_LibraryKey.BP_LibraryKey_C" :`true` "/Game/PickUpObject/BP_LibraryKeyDud.BP_LibraryKeyDud_C" :!type "/Game/PickUpObject/BP_GenericObject Class Reference") "NewEnumerator1" (select `bool` _returnvalue :`false` "/Game/DialogSystem/DialogTree/DialogTree_FoundObject.DialogTree_FoundObject" :`true` "/Game/DialogSystem/DialogTree/DialogTree_FoundDudKey.DialogTree_FoundDudKey" :!type "BehaviorTree Object Reference") true null))
        (set `self.SpawnedKey` _returnvalue_2)
        (`KismetArrayLibrary.Array_RemoveItem` _keylocations _output)))))

(fn `UserConstructionScript`)