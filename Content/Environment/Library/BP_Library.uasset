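; BP_Library is a library environment prop that assembles a bookshelf with randomized meshes for visual variety.
; The construction script independently picks one of three book meshes for each of the two book components and one of two meshes for the shelf.
; The random picks are unseeded, so the look can change whenever the construction script reruns.
; The event graph holds only disabled stub events, with no runtime logic.
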(fn `UserConstructionScript`
  (`StaticMeshComponent.SetStaticMesh` (`self.Books1`) (select `int` (`KismetMathLibrary.RandomIntegerInRange` 0 2) :`0` "/Game/Environment/Library/SM_Books_Cube_006.SM_Books_Cube_006" :`1` "/Game/Environment/Library/SM_Books_Cube_007.SM_Books_Cube_007" :`2` "/Game/Environment/Library/SM_Books_Cube_008.SM_Books_Cube_008" :!type "StaticMesh Object Reference"))
  (`StaticMeshComponent.SetStaticMesh` (`self.Books`) (select `int` (`KismetMathLibrary.RandomIntegerInRange` 0 2) :`0` "/Game/Environment/Library/SM_Books_Cube_006.SM_Books_Cube_006" :`1` "/Game/Environment/Library/SM_Books_Cube_007.SM_Books_Cube_007" :`2` "/Game/Environment/Library/SM_Books_Cube_008.SM_Books_Cube_008" :!type "StaticMesh Object Reference"))
  (`StaticMeshComponent.SetStaticMesh` (`self.Shelf`) (select `int` (`KismetMathLibrary.RandomIntegerInRange` 0 1) :`0` "/Game/Environment/Library/SM_Libraries_Cube_004.SM_Libraries_Cube_004" :`1` "/Game/Environment/Library/SM_Libraries_Cube_005.SM_Libraries_Cube_005" :!type "StaticMesh Object Reference")))