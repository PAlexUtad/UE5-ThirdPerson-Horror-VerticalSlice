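; Spawner that places BP_VineGhoul enemies with the BT_RoamChase behavior tree at random level waypoints.
; BeginPlay caches every BP_Waypoint; Spawn, not called from BeginPlay, recounts live ghouls, shuffles waypoints and spawns one with a particle burst.
; Spawn re-calls itself after a fixed delay, but the loop ends once the enemy cap is reached or no waypoints exist.
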(event `self.ReceiveBeginPlay`
  ;[0.1501 1 0] Begin Play Get all waypoints for spawning
  (bind _outactors (`GameplayStatics.GetAllActorsOfClass` "/Game/ThirdPerson/Blueprints/AI/BP_Waypoint.BP_Waypoint_C"))
  (set `self.Waypoints` _outactors))

(event `Spawn`
  (bind _waypoints (`self.Waypoints`))
  (bind _returnvalue (`self.K2_GetActorLocation` (`|GetArrayItem` (`self.Waypoints`))))
  ;[1 0.67 0.6666] Spawn Zombie: get random waypoint and spawn ai with an emitter
  (`self.CheckEnemyAmount`)
  (if (and (`KismetArrayLibrary.Array_IsNotEmpty` _waypoints) (< (`KismetArrayLibrary.Array_Length` (`self.SpawnedEnemies`)) (`self.MaxEnemyCount`)))
    (`KismetArrayLibrary.Array_Shuffle` _waypoints)
    (bind _returnvalue_2 (`AIBlueprintHelperLibrary.SpawnAIFromClass` "/Game/ThirdPerson/Blueprints/VineGhoul/BP_VineGhoul.BP_VineGhoul_C" "/Game/ThirdPerson/Blueprints/AI/BT_RoamChase.BT_RoamChase" _returnvalue (struct) false null))
    (`/Engine/EditorBlueprintResources/StandardMacros.IsValid` _returnvalue_2
      (:`Is Valid`
        (`GameplayStatics.SpawnEmitterAtLocation` "/Game/VFX_Toolkit_V1/ParticleSystems/356Days/Par_BombWaker.Par_BombWaker" _returnvalue (struct) (0.6 0.6 0.6)))
      (:`Is Not Valid`
        _))
    (`KismetSystemLibrary.Delay` 5.0)
    (`self.Spawn`)))

(event `CheckEnemyAmount`
  ;[0.3571 0.2882 1] Check how many enemies are on the map (take into account those killed by player)
  (bind _outactors (`GameplayStatics.GetAllActorsOfClass` "/Game/ThirdPerson/Blueprints/VineGhoul/BP_VineGhoul.BP_VineGhoul_C"))
  (set `self.SpawnedEnemies` _outactors))

(fn `UserConstructionScript`)