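; Interactable door that switches the game to another level, optionally locked behind a key in the player's obtained keys.
; On interact, it plays a sound and stores spawn position, player rotation, outfit and held object in BP_GameInstance to carry across the load.
; It then disables input, optionally fades out music, and opens the level by name once the WG_Fade fade-in delay ends.
; Without the key, it plays a locked-door sound.
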(event `self.ReceiveBeginPlay`
  ;[0.2449 1 0] BeginPlay
  (`parent.ReceiveBeginPlay`)
  (bind _asbp_game_instance (cast `/Game/ThirdPerson/Blueprints/BP_GameInstance` (`GameplayStatics.GetGameInstance`)))
  (set `self.As BP Game Instance` _asbp_game_instance)
  (if (`self.B_IsLocked`)
    (bind _asbp_third_person_character (cast `/Game/ThirdPerson/Blueprints/BP_ThirdPersonCharacter` (`GameplayStatics.GetPlayerPawn` 0)))
    (set `self.PlayerRef` _asbp_third_person_character)))

(event `EnhancedInput|/Game/ThirdPerson/Input/Actions/IA_Interact`
  (params (ActionValue :type Boolean) (ElapsedSeconds :type "Float (double-precision)") (TriggeredSeconds :type "Float (double-precision)") (InputAction :type "InputAction Object Reference" :default "/Game/ThirdPerson/Input/Actions/IA_Interact.IA_Interact"))
  (bind _returnvalue (`GameplayStatics.GetPlayerPawn` 0))
  (bind _as_bp_game_instance (`self.As BP Game Instance`))
  (bind _playerref (`self.PlayerRef`))
  ;[1 1 1] ChangeLevelWithFade
  (:`Started`
    (if (not (`self.B_IsLocked`))
      (`|ExecutionSequence` :!label _label
        (:`then_0`
          (`GameplayStatics.PlaySound2D` (select `bool` (`self.BusStopSound`) :`false` "/Game/SFX/SC_DoorOpen.SC_DoorOpen" :`true` "/Game/SFX/WAV/Dialogue/PauseMenuOpen.PauseMenuOpen" :!type "SoundBase Object Reference") 1.0 1.0 0.0 null null)
          (set `/Game/ThirdPerson/Blueprints/BP_GameInstance.R_StartRotation` (`self.K2_GetActorRotation` _returnvalue) _as_bp_game_instance)
          (set `/Game/ThirdPerson/Blueprints/BP_GameInstance.V_StartPosition` (`self.NewPosition`) _as_bp_game_instance)
          (bind _asbp_third_person_character (cast `/Game/ThirdPerson/Blueprints/BP_ThirdPersonCharacter` _returnvalue))
          (set `/Game/ThirdPerson/Blueprints/BP_GameInstance.U_OutfitIndex` (`/Game/ThirdPerson/Blueprints/BP_ThirdPersonCharacter.U_CurrentOutfit_Index` _asbp_third_person_character) _as_bp_game_instance)
          (set `/Game/ThirdPerson/Blueprints/BP_GameInstance.BP_$ObjectInHand` (`/Game/ThirdPerson/Blueprints/BP_ThirdPersonCharacter.BP_$ObjectInHand` _asbp_third_person_character) _as_bp_game_instance)
          (`self.DisableInput` _returnvalue (`GameplayStatics.GetPlayerController` 0)))
        (:`then_1`
          (if (`self. B_DoesFadeOutMusic`)
            (`/Game/ThirdPerson/Blueprints/BP_GameInstance.CE_FadeOutMusic` (`self.As BP Game Instance`))))
        (:`then_2`
          (bind _returnvalue_2 (`|CreateWidget` "/Game/Environment/WG_Fade.WG_Fade_C"))
          (`UserWidget.AddToViewport` _returnvalue_2 0)
          (`/Game/Environment/WG_Fade.FadeIn` _returnvalue_2)
          (`KismetSystemLibrary.Delay` (`WidgetAnimation.GetEndTime` (`/Game/Environment/WG_Fade.Fade` _returnvalue_2)))
          (`GameplayStatics.OpenLevel` (`self.Level Name`))))
      (else
        (`/Engine/EditorBlueprintResources/StandardMacros.IsValid` _playerref
          (:`Is Valid`
            (if (!= (`KismetArrayLibrary.Array_Find` (`/Game/ThirdPerson/Blueprints/BP_ThirdPersonCharacter.L_Keys_Obtained` _playerref) (`self.KeyObject`)) -1)
              (goto _label)
              (else
                (`GameplayStatics.PlaySoundAtLocation` "/Game/SFX/SC_DoorLocked.SC_DoorLocked" (`self.K2_GetActorLocation`) (struct) 1.0 1.0 0.0 null null null null)))))))))

(fn `UserConstructionScript`)