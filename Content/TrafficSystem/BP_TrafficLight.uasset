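; Traffic light actor that cycles red, orange and green by swapping emissive materials on its mesh slots.
; A self-calling event loop with delays starts at BeginPlay and advances the phase, with red duration set by a variable.
; A box has query collision on red and orange and none on green.
; When LightActor's pitch rises above a threshold, serving as a time-of-day check, it blinks orange instead, leaving the box unchanged.
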(event `self.ReceiveBeginPlay`
  ;[0.5967 1 0.3263] Begin Play
  (`KismetSystemLibrary.Delay` 0.2)
  (`self.CE_ChangeLight`))

(event `CE_ChangeLight`
  (bind _sm_cityprops_cube_011 (`self.SM_CityProps_Cube_011`))
  (bind _index (`self.Index`))
  (bind _sm_cityprops_cube_011_2 (`self.SM_CityProps_Cube_011`))
  (bind (_returnvalue_roll _returnvalue_pitch) (`KismetMathLibrary.BreakRotator` (`self.K2_GetActorRotation` (`self.LightActor`))))
  ;[1 0.1418 0.1319] Change behavior based on time of day
  (if (> _returnvalue_pitch -6.0)
    (`PrimitiveComponent.SetMaterial` _sm_cityprops_cube_011 2 "/Game/Environment/Materials/MI_EmissiveOFF_Inst.MI_EmissiveOFF_Inst")
    (`PrimitiveComponent.SetMaterial` _sm_cityprops_cube_011 3 "/Game/Environment/Materials/MI_EmissiveOFF_Inst.MI_EmissiveOFF_Inst")
    (`PrimitiveComponent.SetMaterial` _sm_cityprops_cube_011 4 "/Game/Environment/Materials/MI_EmissiveOFF_Inst.MI_EmissiveOFF_Inst")
    (`KismetSystemLibrary.Delay` 0.5)
    (`PrimitiveComponent.SetMaterial` _sm_cityprops_cube_011 3 "/Game/Environment/Materials/MI_Emissive_ORANGE.MI_Emissive_ORANGE")
    (`KismetSystemLibrary.Delay` 0.5)
    (else
      (bind _result (`/Engine/EditorBlueprintResources/StandardMacros.IncrementInt` (`self.Index`))
        (:`  `
          (if (> _result 2)
            (set `self.Index` 0))
          (`PrimitiveComponent.SetMaterial` _sm_cityprops_cube_011_2 2 "/Game/Environment/Materials/MI_EmissiveOFF_Inst.MI_EmissiveOFF_Inst")
          (`PrimitiveComponent.SetMaterial` _sm_cityprops_cube_011_2 3 "/Game/Environment/Materials/MI_EmissiveOFF_Inst.MI_EmissiveOFF_Inst")
          (`PrimitiveComponent.SetMaterial` _sm_cityprops_cube_011_2 4 "/Game/Environment/Materials/MI_EmissiveOFF_Inst.MI_EmissiveOFF_Inst")
          (`PrimitiveComponent.SetMaterial` _sm_cityprops_cube_011_2 (+ (`self.Index`) 2) (select `int` _index :`0` "/Game/Environment/Materials/MI_Emissive_RED.MI_Emissive_RED" :`1` "/Game/Environment/Materials/MI_Emissive_ORANGE.MI_Emissive_ORANGE" :`2` "/Game/Environment/Materials/MI_Emissive_GREEN.MI_Emissive_GREEN" :!type "MaterialInterface Object Reference"))
          (`PrimitiveComponent.SetCollisionEnabled` (`self.Box`) (select `int` _index :`0` "QueryOnly" :`1` "QueryOnly" :`2` "NoCollision" :!type "ECollisionEnabled Enum"))
          (`KismetSystemLibrary.Delay` (select `int` (`self.Index`) :`0` (`self.RedLightTime`) :`1` 2.0 :`2` 10.0))))))
  (`self.CE_ChangeLight`))

(fn `UserConstructionScript`)