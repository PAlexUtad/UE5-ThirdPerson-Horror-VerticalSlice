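; Traffic car that gets a random mesh, speed and sounds, follows a spline via a Timeline, then decrements the spline's count and destroys itself.
; A looping timer sphere-traces ahead for cars, traffic lights and players, playing or reversing a deceleration Timeline that drives the follow play rate.
; It sends its speed to cars ahead and honks at blocking players.
; Engine pitch tracks speed, and headlights toggle by time of day.
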(event `self.ReceiveBeginPlay`
  (bind _spline (`self.Spline`))
  (bind _returnvalue_location (`KismetMathLibrary.BreakTransform` (`SplineComponent.GetTransformAtTime` (`/Game/TrafficSystem/BP_SplineRoad.Spline` _spline) 0.0 "World" false false)))
  ;[1 0.673 0.5962] Begin Play and follow spline
  (`KismetArrayLibrary.Array_Shuffle` (`self.CarMeshes`))
  (`SkeletalMeshComponent.SetSkeletalMeshAsset` (`self.SkeletalMesh`) (`|GetArrayItem` (`self.CarMeshes`)))
  (`/Engine/EditorBlueprintResources/StandardMacros.IsValid` _spline
    (:`Is Valid`
      (`self.K2_SetActorLocation` _returnvalue_location)
      (bind _output_get (set `self.OriginalSpeed` (`KismetMathLibrary.RandomFloatInRange` 0.5 0.65)))
      (set `self.CurrentSpeed` _output_get)
      (`TimelineComponent.SetPlayRate` (`self.Follow`) _output_get)
      (`self.FollowSpline`)
      (set `self.RandomPitchMulitplier` (`KismetMathLibrary.RandomFloatInRange` 0.5 3.0))
      (bind _returnvalue (`GameplayStatics.SpawnSoundAttached` "/Game/SFX/SC_CarEngine.SC_CarEngine" (`self.SkeletalMesh`) "None" (0.0 0.0 0.0) (struct) "KeepRelativeOffset" false 1.0 1.0 0.0 null null))
      (set `self.EngineSound` _returnvalue)
      (set `self.HonkSound` (select `int` (`KismetMathLibrary.RandomIntegerInRange` 0 2) :`0` "/Game/SFX/SC_CarHonk.SC_CarHonk" :`1` "/Game/SFX/SC_CarHonk2.SC_CarHonk2" :`2` "/Game/SFX/SC_CarHonk3.SC_CarHonk3" :!type "SoundBase Object Reference"))
      (`KismetSystemLibrary.K2_SetTimerDelegate` (delegate `CheckFront`) 0.1 true))))

(event `FollowSpline`
  (bind _enginesound (`self.EngineSound`))
  ;[1 0.673 0.5962] Begin Play and follow spline
  (bind (_direction _newtrack_0) (`Timeline|Follow` :!via `PlayFromStart`)
    (:`Update`
      (bind (_returnvalue_location _returnvalue_rotation) (`KismetMathLibrary.BreakTransform` (`SplineComponent.GetTransformAtTime` (`/Game/TrafficSystem/BP_SplineRoad.Spline` (`self.Spline`)) _newtrack_0 "World" true false)))
      (`self.K2_SetActorLocation` _returnvalue_location)
      (`self.K2_SetActorRotation` _returnvalue_rotation)
      (`/Engine/EditorBlueprintResources/StandardMacros.IsValid` _enginesound
        (:`Is Valid`
          (`AudioComponent.SetPitchMultiplier` _enginesound (* (`self.CurrentSpeed`) (`self.RandomPitchMulitplier`))))))
    (:`Finished`
      (`/Game/TrafficSystem/BP_SplineRoad.DecreaseAmt` (`self.Spline`))
      (`self.K2_DestroyActor`))))

(event `/Game/TrafficSystem/INT_SplineCar.ChangeSpeed`
  (params (`New Speed` :type "Float (double-precision)"))
  ;[1 0.673 0.5962] Begin Play and follow spline
  (set `self.OriginalSpeed` `New Speed`))

(event `Deccelarate`
  ;[0.5075 0.5194 1] Change Speed (change play rate of FOLLOW timeline)
  (set `self.TargetSpeed` 0.0)
  (bind (_direction _newtrack_0) (`Timeline|Decc` :!via `PlayFromStart` :!label _label)
    (:`Update`
      (bind _output_get (set `self.CurrentSpeed` (`KismetMathLibrary.Lerp` (`self.OriginalSpeed`) (`self.TargetSpeed`) _newtrack_0)))
      (`TimelineComponent.SetPlayRate` (`self.Follow`) _output_get))))

(event `StopDecc`
  ;[0.5075 0.5194 1] Change Speed (change play rate of FOLLOW timeline)
  (goto _label :!via `Stop`))

(event `Accelerate`
  ;[0.5075 0.5194 1] Change Speed (change play rate of FOLLOW timeline)
  (set `self.TargetSpeed` 0.0)
  (goto _label :!via `Reverse`))

(event `CheckFront`
  (bind _returnvalue (`self.K2_GetActorLocation`))
  (bind _returnvalue_2 (`self.GetActorForwardVector`))
  (bind _returnvalue_3 (`self.K2_GetActorLocation`))
  (bind _returnvalue_4 (`self.GetActorForwardVector`))
  ;[1 0.405 0.1729] Check what's in front of the car (Player, traffic light, other cars)
  (bind (_outhits _returnvalue_5) (`KismetSystemLibrary.SphereTraceMulti` (+ _returnvalue (* _returnvalue_2 50.0)) (+ _returnvalue (* _returnvalue_2 700.0)) 100.0 "TraceTypeQuery3"))
  (for _array_element _outhits
    (if (and _returnvalue_5 (not (`self.isDecc`)))
      (bind (_bblockinghit _binitialoverlap _time _distance _location _impactpoint _normal _impactnormal _physmat _hitactor) (`GameplayStatics.BreakHitResult` _array_element))
      (if (`KismetSystemLibrary.DoesImplementInterface` _hitactor "/Game/TrafficSystem/INT_SplineCar.INT_SplineCar_C")
        (message `/Game/TrafficSystem/INT_SplineCar.ChangeSpeed` _hitactor (`self.OriginalSpeed`))
        (`self.Deccelarate` :!label _label_2)
        (set `self.isDecc` true)
        (elif (or (`KismetSystemLibrary.DoesImplementInterface` _hitactor "/Game/TrafficSystem/INT_TrafficLight.INT_TrafficLight_C") (`KismetSystemLibrary.DoesImplementInterface` _hitactor "/Game/ThirdPerson/Blueprints/Interfaces/BPINT_Player.BPINT_Player_C"))
          (goto _label_2)))
      (else
        (`KismetSystemLibrary.Delay` 1.0 :!label _label_3)
        (if (< (`self.CurrentSpeed`) 0.3)
          (bind (_outhits_2 _returnvalue_6) (`KismetSystemLibrary.SphereTraceMulti` (+ _returnvalue_3 (* _returnvalue_4 50.0)) (+ _returnvalue_3 (* _returnvalue_4 700.0)) 100.0 "TraceTypeQuery3"))
          (if _returnvalue_6
            (for _array_element_2 _outhits_2
              (bind (_bblockinghit_2 _binitialoverlap_2 _time_2 _distance_2 _location_2 _impactpoint_2 _normal_2 _impactnormal_2 _physmat_2 _hitactor_2) (`GameplayStatics.BreakHitResult` _array_element_2))
              (bind _returnvalue_7 (`KismetSystemLibrary.DoesImplementInterface` _hitactor_2 "/Game/ThirdPerson/Blueprints/Interfaces/BPINT_Player.BPINT_Player_C"))
              (if (or (`KismetSystemLibrary.DoesImplementInterface` _hitactor_2 "/Game/TrafficSystem/INT_SplineCar.INT_SplineCar_C") (`KismetSystemLibrary.DoesImplementInterface` _hitactor_2 "/Game/TrafficSystem/INT_TrafficLight.INT_TrafficLight_C") _returnvalue_7)
                (if _returnvalue_7
                  (`/Engine/EditorBlueprintResources/StandardMacros.DoOnce` false :!label _label_4
                    (:`Completed`
                      (`GameplayStatics.PlaySoundAtLocation` (`self.HonkSound`) (`self.K2_GetActorLocation`) (struct) 1.0 1.0 0.0 null null null null)
                      (`KismetSystemLibrary.Delay` 2.0)
                      (goto _label_4 :!via `Reset`)))
                  (else
                    (goto _label_4 :!via `Reset`)))
                (else
                  (`self.Accelerate` :!label _label_5)
                  (set `self.isDecc` false :!label _label_6)
                  (goto _label_4 :!via `Reset`))))
            (else
              (goto _label_5)))
          (else
            (goto _label_6))))))
  (goto _label_3))

(event `ToggleHeadlights`
  ;[1 0.405 0.1729] Check what's in front of the car (Player, traffic light, other cars)
  ;;[1 1 1] Turn on lights if it's night
  (if (`self.IsDaytime`)
    (`LightComponent.SetIntensity` (`self.SpotLight`) 0.0)
    (`LightComponent.SetIntensity` (`self.SpotLight1`) 0.0)
    (else
      (`LightComponent.SetIntensity` (`self.SpotLight`) 10000.0)
      (`LightComponent.SetIntensity` (`self.SpotLight1`) 10000.0))))

(fn `UserConstructionScript`)