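; BP_SaveCoffeeMachine is an interactable coffee machine that serves as a save point.
; It builds on a parent Blueprint, setting its collision radius at construction and the text of its W_Interact widget on Begin Play.
; When IA_Interact starts, it casts the player pawn to BP_ThirdPersonCharacter and calls CESave, leaving the save logic to the character.
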(event `self.ReceiveBeginPlay`
  ;[0.1839 1 0] Begin Play
  (`parent.ReceiveBeginPlay`)
  (bind _asw_interact (cast `/Game/DialogSystem/W_Interact` (`WidgetComponent.GetWidget` (`self.Widget`))))
  (set `TextBlock.Text` (`self.T_SaveText`) (`/Game/DialogSystem/W_Interact.TextBlock_24` _asw_interact)))

(event `EnhancedInput|/Game/ThirdPerson/Input/Actions/IA_Interact`
  (params (ActionValue :type Boolean) (ElapsedSeconds :type "Float (double-precision)") (TriggeredSeconds :type "Float (double-precision)") (InputAction :type "InputAction Object Reference" :default "/Game/ThirdPerson/Input/Actions/IA_Interact.IA_Interact"))
  ;[0.2719 0.7878 1] On Interaction
  (:`Started`
    (bind _asbp_third_person_character (cast `/Game/ThirdPerson/Blueprints/BP_ThirdPersonCharacter` (`GameplayStatics.GetPlayerPawn` 0)))
    (`/Game/ThirdPerson/Blueprints/BP_ThirdPersonCharacter.CE_Save` _asbp_third_person_character)))

(fn `UserConstructionScript`
  (`parent.UserConstructionScript`)
  (set `self.CollisionRadius` 60.0))