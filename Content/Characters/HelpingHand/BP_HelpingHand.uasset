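; BP_HelpingHand is an interactable character that offers dialogue to the player.
; On BeginPlay it hides its prompt widget and passes its DialogueTree to the DialogComponent.
; When BP_ThirdPersonCharacter overlaps the InteractionCollision, it shows the widget and registers the DialogComponent as that character's in-range interactable.
; Leaving the collision clears that reference and hides the widget.
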(event `self.ReceiveBeginPlay`
  (`parent.ReceiveBeginPlay`)
  (`SceneComponent.SetVisibility` (`self.Widget`) false false)
  (set `/Game/DialogSystem/DialogComponent.DialogTree` (`self.DialogueTree`) (`self.DialogComponent`)))

(event `self.InteractionCollision.OnComponentBeginOverlap`
  (params (OverlappedComponent :type "PrimitiveComponent Object Reference") (OtherActor :type "Actor Object Reference") (OtherComp :type "PrimitiveComponent Object Reference") (OtherBodyIndex :type Integer) (bFromSweep :type Boolean) (SweepResult :type "HitResult Structure (by ref)"))
  (bind _asbp_third_person_character (cast `/Game/ThirdPerson/Blueprints/BP_ThirdPersonCharacter` OtherActor))
  (bind _output_get (set `self.As BP Third Person Character` _asbp_third_person_character))
  (`SceneComponent.SetVisibility` (`self.Widget`) true false)
  (set `/Game/ThirdPerson/Blueprints/BP_ThirdPersonCharacter.I_InteractInRange` (`self.DialogComponent`) _output_get))

(event `self.InteractionCollision.OnComponentEndOverlap`
  (params (OverlappedComponent :type "PrimitiveComponent Object Reference") (OtherActor :type "Actor Object Reference") (OtherComp :type "PrimitiveComponent Object Reference") (OtherBodyIndex :type Integer))
  (bind _asbp_third_person_character (cast `/Game/ThirdPerson/Blueprints/BP_ThirdPersonCharacter` OtherActor))
  (set `/Game/ThirdPerson/Blueprints/BP_ThirdPersonCharacter.I_InteractInRange` null _asbp_third_person_character)
  (set `self.As BP Third Person Character` null)
  (`SceneComponent.SetVisibility` (`self.Widget`) false false))

(fn `UserConstructionScript`
  (`parent.UserConstructionScript`))